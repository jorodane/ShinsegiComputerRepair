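; BP_SnackBag is a selectable, interactable snack bag object that changes size when the player interacts with it.
; Interact scales the actor up by 10 percent when the main hand is the right hand, and down by 10 percent otherwise.
; The selectable functions always report it as selectable and return the actor itself, with empty name and action text.
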(event EventBeginPlay)

(event Collision|EventActorBeginOverlap
  (params (OtherActor :type Actor%20Object%20Reference)))

(event EventTick
  (params (DeltaSeconds :type Float%20%28single-precision%29)))

(event EventInteract
  (params (Info :type BS%20Select%20Checker%20Structure))
  (bind _returnvalue (Transformation|GetActorScale3D))
  (if (Variables|/Game/1_Main/Blueprints/Objects/BP_Hand.BP_Hand_C|GetIsRightHand (.mainhand Info))
    (Transformation|SetActorScale3D (* _returnvalue 1.1))
    (else
      (Transformation|SetActorScale3D (* _returnvalue 0.9)))))

(fn ConstructionScript)

(fn GetSelectable
  (params (Info :type BS%20Select%20Checker%20Structure))
  (return true))

(fn GetSelectableActionName
  (params (Info :type BS%20Select%20Checker%20Structure))
  (return ""))

(fn GetSelectableActor
  (return self))

(fn GetSelectableName
  (params (Info :type BS%20Select%20Checker%20Structure))
  (return ""))